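; BP_Block_Suspicious_Sand is a block Blueprint that hurts the first-person character while it overlaps the block's Box collision.
; On overlap begin it stores the player, applies a small initial hit and starts a looping timer that deals heavier damage at a fixed interval.
; On overlap end it clears that timer, stopping the damage.
; BeginPlay and the construction script only call their parents.
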(event `self.ReceiveBeginPlay`
  (`parent.ReceiveBeginPlay`))

(event `self.Box.OnComponentBeginOverlap`
  (params (OverlappedComponent :type "PrimitiveComponent Object Reference") (OtherActor :type "Actor Object Reference") (OtherComp :type "PrimitiveComponent Object Reference") (OtherBodyIndex :type Integer) (bFromSweep :type Boolean) (SweepResult :type "HitResult Structure (by ref)"))
  ;[0.05127 0.05127 0.05127] Damage player if player enters and stays in collision with block
  (bind _asbp_first_person_character (cast `/Game/FirstPerson/Blueprints/BP_FirstPersonCharacter` OtherActor))
  (bind _output_get (set `self.PlayerRef` _asbp_first_person_character))
  (`/Game/FirstPerson/Blueprints/BP_FirstPersonCharacter.Damage` _output_get 2)
  (bind _returnvalue (`KismetSystemLibrary.K2_SetTimerDelegate` (delegate `LoopDamage`) 0.75 true))
  (set `self.TimerHandle` _returnvalue))

(event `LoopDamage`
  ;[0.05127 0.05127 0.05127] Damage player if player enters and stays in collision with block
  (`/Game/FirstPerson/Blueprints/BP_FirstPersonCharacter.Damage` (`self.PlayerRef`) 11))

(event `self.Box.OnComponentEndOverlap`
  (params (OverlappedComponent :type "PrimitiveComponent Object Reference") (OtherActor :type "Actor Object Reference") (OtherComp :type "PrimitiveComponent Object Reference") (OtherBodyIndex :type Integer))
  ;[0.05127 0.05127 0.05127] Reset timer
  (cast `/Game/FirstPerson/Blueprints/BP_FirstPersonCharacter` OtherActor)
  (`KismetSystemLibrary.K2_ClearAndInvalidateTimerHandle` (`self.TimerHandle`)))

(fn `UserConstructionScript`
  (`parent.UserConstructionScript`))