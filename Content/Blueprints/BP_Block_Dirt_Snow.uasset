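; BP_Block_Dirt_Snow is a snowy dirt block for a block game that the player can break and collect.
; BeginPlay makes dynamic instances of its three materials and sets the destroy timeline's rate.
; StartDestroy animates their DestroyAmount parameter, while StopDestroy cancels and resets it.
; When the timeline finishes, the block is removed from GI_BlockGame, its class is added to the first-person character's inventory, and the actor is destroyed.
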(event `self.ReceiveBeginPlay`
  (bind _block (`self.Block`))
  ;[0.05127 0.05127 0.05127] Create a dynamic material instance on all materials of the array and set play rate
  (`TimelineComponent.SetPlayRate` (`self.Destroy Timeline`) (`self.DestroyRate`))
  (for _index (range 3)
    (bind _returnvalue (`PrimitiveComponent.CreateDynamicMaterialInstance` _block _index (`PrimitiveComponent.GetMaterial` _block _index) "None"))
    (`KismetArrayLibrary.Array_Add` (`self.Materials`) _returnvalue)))

(event `self.StartDestroy`
  ;[0.05127 0.05127 0.05127] Edit the dynamic material on all materials of the array to start or stop a destroy action
  (bind (_direction _destroyamount) (`Timeline|Timeline` :!via `PlayFromStart` :!label _label)
    (:`Update`
      (`MaterialInstanceDynamic.SetScalarParameterValue` (`self.Materials`) "DestroyAmount" _destroyamount))
    (:`Finished`
      (`/Game/FirstPerson/Blueprints/GI_BlockGame.RemoveBlock` (cast `/Game/FirstPerson/Blueprints/GI_BlockGame` (`GameplayStatics.GetGameInstance`) :!pure true) (`SceneComponent.K2_GetComponentLocation` (`self.Block`)))
      (bind _asbp_first_person_character (cast `/Game/FirstPerson/Blueprints/BP_FirstPersonCharacter` (`GameplayStatics.GetPlayerCharacter` 0)))
      (`/Game/FirstPerson/Blueprints/BP_FirstPersonCharacter.AddBlockToInventory` _asbp_first_person_character (`GameplayStatics.GetObjectClass` self))
      (`self.K2_DestroyActor`))))

(event `self.StopDestroy`
  ;[0.05127 0.05127 0.05127] Edit the dynamic material on all materials of the array to start or stop a destroy action
  (`MaterialInstanceDynamic.SetScalarParameterValue` (`self.Materials`) "DestroyAmount" 0.0) ; Resetting the DestroyAmount Parameter
  (goto _label :!via `Stop`))

(fn `UserConstructionScript`
  (`parent.UserConstructionScript`))